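; Gameplay ability that casts a fire bolt projectile toward the point under the mouse cursor.
; After committing, it gets mouse target data, turns the avatar to face the hit location through CombatInterface, and plays the cast montage.
; An Event.Montage.Fire gameplay event times the SpawnProjectile call to the animation.
; The ability ends when the montage completes, blends out, is interrupted or is cancelled.
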(event `self.K2_ActivateAbility`
  (`self.K2_CommitAbility`)
  (bind (_asynctaskproxy _datahandle) (`TargetDataUnderMouse.CreateTargetDataUnderMouse`)
    (:`ValidData`
      (set `self.ProjectileTargetLocation` (`.Location` (`GameplayStatics.BreakHitResult` (`AbilitySystemBlueprintLibrary.GetHitResultFromTargetData` _datahandle))))
      (bind _ascombat_interface (cast `CombatInterface` (`self.GetAvatarActorFromActorInfo`)))
      (`CombatInterface.UpdateFacingTarget` _ascombat_interface (`self.ProjectileTargetLocation`))
      (`AbilityTask_PlayMontageAndWait.CreatePlayMontageAndWaitProxy` "None" "/Game/Retatgeting/AM_Cast_FireBolt.AM_Cast_FireBolt" 1.0 "None" false
        (:`then`
          (`AbilityTask_WaitGameplayEvent.WaitGameplayEvent` (struct :`TagName` "Event.Montage.Fire") null
            (:`EventReceived`
              (`self.SpawnProjectile` (`self.ProjectileTargetLocation`)))))
        (:`OnCompleted`
          (`self.K2_EndAbility` :!label _label))
        (:`OnBlendOut`
          (goto _label))
        (:`OnInterrupted`
          (goto _label))
        (:`OnCancelled`
          (goto _label))))))