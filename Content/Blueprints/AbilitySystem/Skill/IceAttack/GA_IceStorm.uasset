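; GA_IceStorm is a gameplay ability that casts an ice storm area effect at the location under the mouse cursor.
; On activation it commits, gets the hit location from mouse target data and turns the avatar toward it through CombatInterface.
; It plays a short cast montage and waits for the montage fire gameplay event, then spawns the area effect at the target and ends the ability.
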(event `self.K2_ActivateAbility`
  (`self.K2_CommitAbility`)
  (bind (_asynctaskproxy _datahandle) (`TargetDataUnderMouse.CreateTargetDataUnderMouse`)
    (:`ValidData`
      (set `self.GetTargetLocation` (`.Location` (`GameplayStatics.BreakHitResult` (`AbilitySystemBlueprintLibrary.GetHitResultFromTargetData` _datahandle))))
      (bind _ascombat_interface (cast `CombatInterface` (`self.GetAvatarActorFromActorInfo`)))
      (`CombatInterface.UpdateFacingTarget` _ascombat_interface (`self.GetTargetLocation`))
      (`AbilityTask_PlayMontageAndWait.CreatePlayMontageAndWaitProxy` "None" "/Game/Retatgeting/Cast_ArcaneShards_Short_Montage.Cast_ArcaneShards_Short_Montage"
        (:`then`
          (`AbilityTask_WaitGameplayEvent.WaitGameplayEvent` (struct :`TagName` "Event.Montage.Fire") null
            (:`EventReceived`
              (`self.SpawnAreaEffect` (`self.GetTargetLocation`))
              (`self.K2_EndAbility`))))))))